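; Riddle challenge manager, an unfinished skeleton for timing riddle phases.
; Once HasBegun is set, Tick adds delta time to Timer only if instructions are already displayed or Timer has reached InstructionsDuration.
; The answers-phase check is left unconnected, and BeginRiddle and EndRiddle are empty stubs.
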(event `self.ReceiveTick`
  (params (DeltaSeconds :type "Float (single-precision)"))
  (if (`self.HasBegun`)
    (if (not (and (not (`self.HasDisplayedInstructions`)) (< (`self.Timer`) (`self.InstructionsDuration`))))
      (set `self.Timer` (+ (`self.Timer`) DeltaSeconds)))))

(fn `BeginRiddle`)

(fn `EndRiddle`)

(fn `UserConstructionScript`)