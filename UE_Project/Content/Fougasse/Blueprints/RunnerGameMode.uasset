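; Game mode for a runner game that builds the level from randomly chosen chunk actors.
; BeginPlay calls AddChunk in a loop to lay the opening stretch of track.
; AddChunk spawns a random class from LevelChunks at NextSpawnPoint, then takes that chunk's attach transform as the next spawn point, chaining pieces end to end.
; The random pick uses LastIndex as an exclusive bound, so the last array entry is never selected.
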(event `self.ReceiveBeginPlay`
  (for _ (range 11)
    (`self.AddChunk`)))

(fn `AddChunk`
  (bind _levelchunk (`self.GetRandomChunk`))
  (bind _returnvalue (`|SpawnActorFromClass` _levelchunk (`self.NextSpawnPoint`) "Undefined" "OverrideRootScale" null null))
  (bind _attachtransform (`/Game/Fougasse/Blueprints/LevelChunks/LevelChunk.GetAttachTransform` _returnvalue))
  (set `self.NextSpawnPoint` _attachtransform))

(fn `GetRandomChunk`
  (returns (LevelChunk :type "/Game/Fougasse/Blueprints/LevelChunks/LevelChunk Class Reference"))
  (bind _levelchunks (`self.LevelChunks`))
  (return (`|GetArrayItem` _levelchunks (`KismetMathLibrary.RandomInteger` (`KismetArrayLibrary.Array_LastIndex` _levelchunks)))))

(fn `UserConstructionScript`)