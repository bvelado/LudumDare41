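; Background actor that keeps its static mesh positioned relative to the runner character, so the backdrop travels with the player.
; On BeginPlay it caches the first BP_RunnerCharacter found in the level.
; Each Tick it moves the mesh to the character capsule's X and Y plus the relative location of a PlayerOffsetLocation component.
; The character's Z is ignored, so height comes only from that offset.
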(event `self.ReceiveBeginPlay`
  (bind _outactors (`GameplayStatics.GetAllActorsOfClass` "/Game/Fougasse/Blueprints/BP_RunnerCharacter.BP_RunnerCharacter_C"))
  (if (> (`KismetArrayLibrary.Array_Length` _outactors) 0)
    (set `self.Character` (`|GetArrayItem` _outactors))))

(event `self.ReceiveTick`
  (params (DeltaSeconds :type "Float (single-precision)"))
  (`SceneComponent.K2_SetWorldLocation` (`self.StaticMeshComponent`) (+ (`SceneComponent.RelativeLocation` (`self.PlayerOffsetLocation`)) (`KismetMathLibrary.MakeVector` (.x (`SceneComponent.K2_GetComponentLocation` (`Character.CapsuleComponent` (`self.Character`)))) (.y (`SceneComponent.K2_GetComponentLocation` (`Character.CapsuleComponent` (`self.Character`)))))) false false))

(fn `UserConstructionScript`)